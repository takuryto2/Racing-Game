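; Player-controlled car pawn that speeds up, turns and strafes through Enhanced Input.
; On BeginPlay it adds the IMC_Default mapping context to the controller of player 0's pawn.
; Tick caches delta time, which the input actions pass with their values to Move, Turn and Strafe, none of which are defined in this graph.
; Speed-up input always calls Move with boosting off.
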(event Input|EnhancedActionEvents|EnhancedInputActionIA_SpeedUp
  (params (ActionValue :type Float%20%28double-precision%29) (ElapsedSeconds :type Float%20%28double-precision%29) (TriggeredSeconds :type Float%20%28double-precision%29) (InputAction :type Input%20Action%20Object%20Reference :default "/Game/Inputs/Actions/IA_SpeedUp.IA_SpeedUp"))
  (Class|CarPawn|Move ActionValue (Variables|Default|GetDelta%20Time) false))

(event Input|EnhancedActionEvents|EnhancedInputActionIA_Turn
  (params (ActionValue :type Float%20%28double-precision%29) (ElapsedSeconds :type Float%20%28double-precision%29) (TriggeredSeconds :type Float%20%28double-precision%29) (InputAction :type Input%20Action%20Object%20Reference :default "/Game/Inputs/Actions/IA_Turn.IA_Turn"))
  (Class|CarPawn|Turn ActionValue (Variables|Default|GetDelta%20Time)))

(event Input|EnhancedActionEvents|EnhancedInputActionIA_Strafe
  (params (ActionValue :type Float%20%28double-precision%29) (ElapsedSeconds :type Float%20%28double-precision%29) (TriggeredSeconds :type Float%20%28double-precision%29) (InputAction :type Input%20Action%20Object%20Reference :default "/Game/Inputs/Actions/IA_Strafe.IA_Strafe"))
  (Class|CarPawn|Strafe ActionValue (Variables|Default|GetDelta%20Time)))

(event EventBeginPlay
  (bind _asplayer_controller (Utilities|Casting|CastToPlayerController (Pawn|GetController (Game|Player|GetPlayerPawn 0))))
  (Utilities|IsValid (PlayerController|LocalPlayerSubsystems|GetEnhancedInputLocalPlayerSubsystem _asplayer_controller)
    (:Is%20Valid
      (Input|AddMappingContext (PlayerController|LocalPlayerSubsystems|GetEnhancedInputLocalPlayerSubsystem _asplayer_controller) "/Game/Inputs/IMC_Default.IMC_Default" 0 "(bIgnoreAllPressedKeysUntilRelease=True,bForceImmediately=False,bNotifyUserSettings=False)"))))

(event EventTick
  (params (DeltaSeconds :type Float%20%28single-precision%29))
  (Variables|Default|SetDelta%20Time DeltaSeconds))

(fn ConstructionScript)